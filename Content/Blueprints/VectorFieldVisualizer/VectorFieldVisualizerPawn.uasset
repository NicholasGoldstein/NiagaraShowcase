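; Camera pawn for a vector field visualizer that spawns a Niagara actor and switches it between low and high quality display.
; Mouse input orbits and zooms a clamped spring arm, except in HQ mode.
; LQ runs a live Niagara system and clears the render target.
; HQ steps ribbon starts across a grid, fast-forwarding and scene-capturing each into a viewport-sized render target shown through a UMG image material.
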(event `self.ReceiveBeginPlay`
  (`SceneComponent.K2_SetWorldLocationAndRotation` :`self` (`self.Scene`) :`NewLocation` (50.0 50.0 50.0))
  (bind _returnvalue (`|SpawnActorFromClass` "/Game/Blueprints/VectorFieldVisualizer/VectorFieldNiagaraActor.VectorFieldNiagaraActor_C" (`KismetMathLibrary.MakeTransform` (0.0 0.0 0.0)) "Undefined" "OverrideRootScale" null null))
  (set `self.VectorFieldVisualizerNiagaraComponent` (`NiagaraActor.NiagaraComponent` _returnvalue))
  (`ActorComponent.SetActive` (`self.VectorFieldVisualizerNiagaraComponent`) true false))

(event `InputAxisKey|MouseY`
  (params (AxisValue :type "Float (single-precision)"))
  (if (not (`self.b_VisualizeHQ`))
    (`SceneComponent.K2_SetWorldRotation` (`self.Scene`) (`KismetMathLibrary.MakeRotator` (.roll (`SceneComponent.K2_GetComponentRotation` (`self.Scene`))) (`KismetMathLibrary.ClampAngle` (+ (.pitch (`SceneComponent.K2_GetComponentRotation` (`self.Scene`))) AxisValue) -80.0 80.0) (.yaw (`SceneComponent.K2_GetComponentRotation` (`self.Scene`)))) false false)))

(event `InputAxisKey|MouseX`
  (params (AxisValue :type "Float (single-precision)"))
  (if (not (`self.b_VisualizeHQ`))
    (`SceneComponent.K2_SetWorldRotation` (`self.Scene`) (`KismetMathLibrary.MakeRotator` (.roll (`SceneComponent.K2_GetComponentRotation` (`self.Scene`))) (.pitch (`SceneComponent.K2_GetComponentRotation` (`self.Scene`))) (+ (.yaw (`SceneComponent.K2_GetComponentRotation` (`self.Scene`))) AxisValue)) false false)))

(event `InputAxisKey|MouseWheelAxis`
  (params (AxisValue :type "Float (single-precision)"))
  (bind _springarm (`self.SpringArm`))
  (if (not (`self.b_VisualizeHQ`))
    (set `SpringArmComponent.TargetArmLength` (`KismetMathLibrary.FClamp` (+ (* -5 AxisValue) (`SpringArmComponent.TargetArmLength` _springarm)) 150.0 250.0) _springarm)))

(fn `UserConstructionScript`)

(fn `VisualizeHQ`
  (returns (Success :type Boolean))
  (bind _vectorfieldvisualizerniagaracomponent (`self.VectorFieldVisualizerNiagaraComponent`))
  (bind (_x _y) (`KismetMathLibrary.BreakVector2D` (`WidgetLayoutLibrary.GetViewportSize`)))
  (set `self.b_VisualizeHQ` true)
  (bind _returnvalue (`KismetRenderingLibrary.CreateRenderTarget2D` (`KismetMathLibrary.FTrunc` _x) (`KismetMathLibrary.FTrunc` _y)))
  (bind _output_get (set `SceneCaptureComponent2D.TextureTarget` _returnvalue (`self.SceneCaptureComponent2D`)))
  (bind _returnvalue_2 (`KismetMaterialLibrary.CreateDynamicMaterialInstance` "/Game/Materials/M_FlipRenderTargetOpacity.M_FlipRenderTargetOpacity"))
  (`MaterialInstanceDynamic.SetTextureParameterValue` _returnvalue_2 "RenderTarget" _output_get)
  (`Image.SetBrushFromMaterial` (`/Game/UMG/VectorFieldVisualizer/UMG_VectorFieldVisualizerInterface.Image_VectorFieldHQ` (`self.UMG_VisualizerInterfaceRef`)) _returnvalue_2)
  (`NiagaraComponent.SetAsset` (`self.VectorFieldVisualizerNiagaraComponent`) "/Game/FX/VectorFieldVisualizer/NS_VectorFieldVisualizerHQ.NS_VectorFieldVisualizerHQ")
  (for _index (range 11)
    (for _index_2 (range 11)
      (`NiagaraComponent.SetNiagaraVariableVec3` _vectorfieldvisualizerniagaracomponent "User.RibbonStartPosition" (`KismetMathLibrary.MakeVector` (* _index 10.0) (* _index_2 10.0)))
      (`NiagaraComponent.ReinitializeSystem` _vectorfieldvisualizerniagaracomponent)
      (`NiagaraComponent.ReinitializeSystem` (`self.VectorFieldVisualizerNiagaraComponent`))
      (`ActorComponent.SetActive` (`self.VectorFieldVisualizerNiagaraComponent`) true false)
      (`NiagaraComponent.AdvanceSimulation` (`self.VectorFieldVisualizerNiagaraComponent`) 50 0.1)
      (`SceneCaptureComponent2D.CaptureScene` (`self.SceneCaptureComponent2D`))))
  (`ActorComponent.SetActive` (`self.VectorFieldVisualizerNiagaraComponent`) false false)
  (return true))

(fn `VisualizeLQ`
  (returns (Success :type Boolean))
  (bind _scenecapturecomponent2d (`self.SceneCaptureComponent2D`))
  (set `self.b_VisualizeHQ` false)
  (`NiagaraComponent.SetAsset` (`self.VectorFieldVisualizerNiagaraComponent`) "/Game/FX/VectorFieldVisualizer/NS_VectorFieldVisualizerLQ.NS_VectorFieldVisualizerLQ")
  (`ActorComponent.SetActive` (`self.VectorFieldVisualizerNiagaraComponent`) true false)
  (`KismetRenderingLibrary.ClearRenderTarget2D` _scenecapturecomponent2d (`SceneCaptureComponent2D.TextureTarget` _scenecapturecomponent2d) (`KismetMathLibrary.MakeColor` 0.0))
  (return true))